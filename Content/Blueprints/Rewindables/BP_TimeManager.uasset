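; BP_TimeManager keeps a shared rewind clock for every actor that implements I_Rewindable.
; It gathers those actors once at BeginPlay, then each Tick moves CurrentTime forward, or backward while IsRewinding is set, clamped between zero and MaxTime, and sends it to each.
; OnRewind and OnUnRewind relay start and stop messages to the same actors, without changing IsRewinding themselves.
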(event `self.ReceiveBeginPlay`
  (bind _outactors (`GameplayStatics.GetAllActorsWithInterface` "/Game/Blueprints/Interfaces/I_Rewindable.I_Rewindable_C"))
  (set `self.Rewindables` _outactors))

(event `self.ReceiveTick`
  (params (DeltaSeconds :type "Float (single-precision)"))
  (`self.CalculateCurrentTime`)
  (for _array_element (`self.Rewindables`)
    (message `/Game/Blueprints/Interfaces/I_Rewindable.SetTimer` _array_element (`self.currentTime`))))

(fn `CalculateCurrentTime`
  (if (`self.IsRewinding?`)
    (set `self.currentTime` (`KismetMathLibrary.FClamp` (- (`self.currentTime`) (`GameplayStatics.GetWorldDeltaSeconds`)) 0.0 (`self.maxTime`)))
    (else
      (set `self.currentTime` (`KismetMathLibrary.FClamp` (+ (`self.currentTime`) (`GameplayStatics.GetWorldDeltaSeconds`)) 0.0 (`self.maxTime`))))))

(fn `OnRewind`
  (for _array_element (`self.Rewindables`)
    (message `/Game/Blueprints/Interfaces/I_Rewindable.OnRewind` _array_element)))

(fn `OnUnRewind`
  (for _array_element (`self.Rewindables`)
    (message `/Game/Blueprints/Interfaces/I_Rewindable.OnUnrewind` _array_element)))

(fn `UserConstructionScript`)