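; BP_RotatingObject is a rewindable child Blueprint that spins its Sphere component continuously.
; Tick adds a local pitch rotation scaled by RotationSpeed and delta time.
; OnRewind and OnUnrewind both negate RotationSpeed, so the spin reverses during a time rewind and flips back afterwards by sign toggling rather than replaying recorded transforms.
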(event `self.ReceiveTick`
  (params (DeltaSeconds :type "Float (single-precision)"))
  ;[0 0 0 0.5] Rotation
  (`SceneComponent.K2_AddLocalRotation` (`self.Sphere`) (`KismetMathLibrary.MakeRotator` 0.0 (* DeltaSeconds (`self.RotationSpeed`))) false false))

(event `/Game/Blueprints/Interfaces/I_Rewindable.OnRewind`
  ;[0 0 0 0.5] TimeRewind Logic
  (set `self.RotationSpeed` (* (`self.RotationSpeed`) -1.0) :!label _label))

(event `/Game/Blueprints/Interfaces/I_Rewindable.OnUnrewind`
  ;[0 0 0 0.5] TimeRewind Logic
  (goto _label))

(fn `UserConstructionScript`
  (`parent.UserConstructionScript`))