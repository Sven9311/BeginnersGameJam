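; Rewindable object Blueprint whose cylinder vanishes and reappears in response to the ReacttoTimer event.
; Each call flips EventPassed, alternately playing and reversing the Vanish timeline, which scales the cylinder between full size and zero.
; When the timeline finishes, it toggles IsVisible and switches collision between query-and-physics and none to match.
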(event `/Game/Blueprints/Interfaces/I_Rewindable.ReactToTimer`
  (if (`self.EventPassed?`)
    (set `self.EventPassed?` (not (`self.EventPassed?`)))
    (bind (_direction _vanishalpha) (`Timeline|Vanish` :!via `Reverse` :!label _label)
      (:`Update`
        (`SceneComponent.SetWorldScale3D` (`self.Cylinder`) (`KismetMathLibrary.VLerp` (1.0 1.0 1.0) (0.0 0.0 0.0) _vanishalpha)))
      (:`Finished`
        (bind _output_get (set `self.isVisible?` (not (`self.isVisible?`))))
        (if _output_get
          (`PrimitiveComponent.SetCollisionEnabled` (`self.Cylinder`) "QueryAndPhysics")
          (else
            (`PrimitiveComponent.SetCollisionEnabled` (`self.Cylinder`) "NoCollision")))))
    (else
      (set `self.EventPassed?` (not (`self.EventPassed?`)))
      (goto _label))))

(fn `UserConstructionScript`
  (`parent.UserConstructionScript`))