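; Rewindable Blueprint that reacts when a supplied time crosses its EventTime, in either forward or backward direction.
; SetTimer passes the time to TriggerEvent and calls ReactToTimer when that check returns true.
; TriggerEvent uses the EventPassed flag to pick the crossing direction: at or after EventTime if not yet passed, at or before it if passed.
; Nothing here updates EventPassed.
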(event `/Game/Blueprints/Interfaces/I_Rewindable.SetTimer`
  (params (Time :type "Float (double-precision)"))
  (if (`self.TriggerEvent?` Time)
    (`/Game/Blueprints/Interfaces/I_Rewindable.ReactToTimer`)))

(fn `TriggerEvent?`
  (params (Time :type "Float (double-precision)"))
  (returns (ShouldReact :type Boolean))
  (return (or (and (<= Time (`self.EventTime`)) (`self.EventPassed?`)) (and (>= Time (`self.EventTime`)) (not (`self.EventPassed?`))))))

(fn `UserConstructionScript`)