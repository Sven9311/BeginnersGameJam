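; Player Blueprint that manages a time-fuel resource for rewinding, forwarding and freezing time.
; Each tick it reads the state of the BP_CustomTimeManager found at BeginPlay, draining fuel during time manipulation and regenerating it during normal play.
; An empty tank forces the manager back to playing and skips regeneration, leaving HandlePickup as the refill path shown here.
; It creates the HUD widget and pushes the fuel fraction to it every tick.
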(event `self.ReceiveBeginPlay`
  (bind _outactors (`GameplayStatics.GetAllActorsOfClass` "/Game/Blueprints/TimeManagement/BP_CustomTimeManager.BP_CustomTimeManager_C"))
  (set `self.TimeManager` (`|GetArrayItem` _outactors))
  (set `self.CurrentTimeFuel` (`self.MaxTimeFuel`))
  (`self.CreateHUDWidget`))

(event `self.ReceiveTick`
  (params (DeltaSeconds :type "Float (single-precision)"))
  (`self.CheckFuel`)
  (`/Game/Widgets/WB_HUD.SetFuelPercent` (`self.HUDWidget`) (`self.CurrentFuelInPercent`)))

(fn `CheckFuel`
  (if (> (`self.CurrentTimeFuel`) 0.0)
    (`self.HandleFuel`)
    (else
      (set `/Game/Blueprints/TimeManagement/BP_CustomTimeManager.ETimeState` "NewEnumerator0" (`self.TimeManager`)))))

(fn `CreateHUDWidget`
  (bind _returnvalue (`|CreateWidget` "/Game/Widgets/WB_HUD.WB_HUD_C" (`GameplayStatics.GetPlayerController` 0)))
  (bind _output_get (set `self.HUDWidget` _returnvalue))
  (`UserWidget.AddToViewport` _output_get 0))

(fn `CurrentFuelInPercent`
  (returns (ReturnValue :type "Float (double-precision)"))
  (return (/ (`self.CurrentTimeFuel`) (`self.MaxTimeFuel`))))

(fn `DrainTimeFuel`
  (set `self.CurrentTimeFuel` (`KismetMathLibrary.FClamp` (- (`self.CurrentTimeFuel`) (* (`self.DrainRate`) (`GameplayStatics.GetWorldDeltaSeconds`))) 0.0 (`self.MaxTimeFuel`)))
  (return))

(fn `HandleFuel`
  (switch `/Game/Blueprints/TimeManagement/CustomTypes/E_TimeState` (`/Game/Blueprints/TimeManagement/BP_CustomTimeManager.ETimeState` (`self.TimeManager`))
    (:`NewEnumerator0`
      (`self.RegenTimeFuel`))
    (:`NewEnumerator1`
      (`self.DrainTimeFuel`))
    (:`NewEnumerator2`
      (`self.DrainTimeFuel`))
    (:`NewEnumerator3`
      (`self.DrainTimeFuel`))))

(fn `HandlePickup`
  (params (RefuelAmount :type "Float (double-precision)"))
  (set `self.CurrentTimeFuel` (`KismetMathLibrary.FClamp` (+ RefuelAmount (`self.CurrentTimeFuel`)) 0.0 (`self.MaxTimeFuel`))))

(fn `RegenTimeFuel`
  (set `self.CurrentTimeFuel` (`KismetMathLibrary.FClamp` (+ (`self.CurrentTimeFuel`) (* (`self.RegenRate`) (`GameplayStatics.GetWorldDeltaSeconds`))) 0.0 (`self.MaxTimeFuel`))))

(fn `UserConstructionScript`)