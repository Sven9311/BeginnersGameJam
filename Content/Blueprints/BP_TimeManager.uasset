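; BP_TimeManager keeps a shared game clock that can run backward for time rewind.
; On BeginPlay it caches every actor implementing the I_Test interface as a rewindable.
; Each Tick it prints the time, steps it forward or backward by world delta seconds depending on IsRewinding, then pushes it to the cached actors through SetTimeMessage.
; Nothing in this graph sets IsRewinding or clamps the time.
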(event `self.ReceiveBeginPlay`
  (bind _outactors (`GameplayStatics.GetAllActorsWithInterface` "/Game/Blueprints/I_Test.I_Test_C"))
  (set `self.Rewindables` _outactors))

(event `self.ReceiveTick`
  (params (DeltaSeconds :type "Float (single-precision)"))
  (`KismetSystemLibrary.PrintString` (`KismetStringLibrary.Conv_DoubleToString` (`self.currentTime`)))
  (if (`self.IsRewinding?`)
    (set `self.currentTime` (- (`self.currentTime`) (`GameplayStatics.GetWorldDeltaSeconds`)))
    (else
      (set `self.currentTime` (+ (`self.currentTime`) (`GameplayStatics.GetWorldDeltaSeconds`)))))
  (for _array_element (`self.Rewindables`)
    (message `/Game/Blueprints/I_Test.SetTime` _array_element (`self.currentTime`))))

(fn `UserConstructionScript`)