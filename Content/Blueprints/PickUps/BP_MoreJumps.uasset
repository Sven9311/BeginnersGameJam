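; BP_MoreJumps is a pickup that permanently grants BP_Player one extra jump by incrementing JumpMaxCount on overlap.
; After collection, a timeline lerps the cube's world scale toward zero, then destroys the actor when it finishes.
; While in the world, it spins around yaw each tick at RotationSpeed, scaled by delta time.
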(event `self.ReceiveActorBeginOverlap`
  (params (OtherActor :type "Actor Object Reference"))
  (bind _cube (`self.Cube`))
  (bind _asbp_player (cast `/Game/Blueprints/Player/BP_Player` OtherActor))
  (`/Engine/EditorBlueprintResources/StandardMacros.IncrementInt` (`Character.JumpMaxCount` _asbp_player)
    (:`  `
      (bind (_direction _shrinkalpha) (`Timeline|Timeline`)
        (:`Update`
          (`SceneComponent.SetWorldScale3D` _cube (`KismetMathLibrary.VLerp` (`SceneComponent.K2_GetComponentScale` _cube) (0.0 0.0 0.0) _shrinkalpha)))
        (:`Finished`
          (`self.K2_DestroyActor`))))))

(event `self.ReceiveTick`
  (params (DeltaSeconds :type "Float (single-precision)"))
  (`self.K2_AddActorWorldRotation` (`KismetMathLibrary.MakeRotator` 0.0 0.0 (* DeltaSeconds (`self.RotationSpeed`)))))

(fn `UserConstructionScript`)