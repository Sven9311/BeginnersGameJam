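; BP_PickUp is a pickup actor that handles the visual collection and respawn of an item.
; It caches the mesh's starting scale on BeginPlay.
; OnPickup plays a timeline that shrinks the mesh to zero, then disables collision and hides the actor.
; OnRespawn reverses this, restoring collision, visibility and the original scale so the actor is reused instead of destroyed.
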(event `self.ReceiveBeginPlay`
  (set `self.InitialSize` (`SceneComponent.K2_GetComponentScale` (`self.PickupMesh`))))

(event `/Game/Blueprints/Interfaces/I_PickUp.OnPickup`
  (bind (_direction _shrinkalpha) (`Timeline|Timeline` :!via `PlayFromStart`)
    (:`Update`
      (`SceneComponent.SetWorldScale3D` (`self.PickupMesh`) (`KismetMathLibrary.VLerp` (`self.InitialSize`) (0.0 0.0 0.0) _shrinkalpha)))
    (:`Finished`
      (`PrimitiveComponent.SetCollisionEnabled` (`self.PickupMesh`) "NoCollision")
      (`self.SetActorHiddenInGame` true))))

(event `/Game/Blueprints/Interfaces/I_PickUp.OnRespawn`
  (`PrimitiveComponent.SetCollisionEnabled` (`self.PickupMesh`) "QueryAndPhysics")
  (`self.SetActorHiddenInGame` false)
  (`SceneComponent.SetWorldScale3D` (`self.PickupMesh`) (`self.InitialSize`)))

(fn `UserConstructionScript`)