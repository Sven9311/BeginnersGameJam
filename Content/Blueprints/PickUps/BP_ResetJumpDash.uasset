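; BP_ResetJumpDash is a spinning pickup that grants the player an extra jump and makes the dash available again.
; On overlap with BP_Player, it increments the player's JumpMaxCount and sets DashAvailable on the player controller.
; A timeline then shrinks both cube meshes by lerping their current scale toward zero, and destroys the actor when finished.
; Tick yaws the actor at RotationSpeed, scaled by delta time.
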(event `self.ReceiveActorBeginOverlap`
  (params (OtherActor :type "Actor Object Reference"))
  (bind _cube1 (`self.Cube1`))
  (bind _cube (`self.Cube`))
  (bind _asbp_player (cast `/Game/Blueprints/Player/BP_Player` OtherActor))
  (`/Engine/EditorBlueprintResources/StandardMacros.IncrementInt` (`Character.JumpMaxCount` _asbp_player)
    (:`  `
      (set `/Game/Blueprints/Controller/BP_GeneralPlayerController.DashAvailable?` true (`/Game/Blueprints/Player/BP_Player.As BP General Player Controller` _asbp_player))
      (bind (_direction _shrinkalpha) (`Timeline|Timeline`)
        (:`Update`
          (`SceneComponent.SetWorldScale3D` _cube (`KismetMathLibrary.VLerp` (`SceneComponent.K2_GetComponentScale` _cube) (0.0 0.0 0.0) _shrinkalpha))
          (`SceneComponent.SetWorldScale3D` _cube1 (`KismetMathLibrary.VLerp` (`SceneComponent.K2_GetComponentScale` _cube1) (0.0 0.0 0.0) _shrinkalpha)))
        (:`Finished`
          (`self.K2_DestroyActor`))))))

(event `self.ReceiveTick`
  (params (DeltaSeconds :type "Float (single-precision)"))
  (`self.K2_AddActorWorldRotation` (`KismetMathLibrary.MakeRotator` 0.0 0.0 (* DeltaSeconds (`self.RotationSpeed`)))))

(fn `UserConstructionScript`)