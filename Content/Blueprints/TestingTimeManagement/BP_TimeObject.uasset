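; BP_TimeObject is an actor that records its own state over time for a custom time manager.
; On BeginPlay it finds the first BP_CustomTimeManager and registers itself as a time actor.
; Each UpdateTime call runs ApplySnapshot, which, despite its name, only appends a snapshot of transform, velocity, visibility and collision flags.
; Snapshot times are rounded to tenths of a unit; the array is never trimmed or played back here.
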(event `self.ReceiveBeginPlay`
  (bind _outactors (`GameplayStatics.GetAllActorsOfClass` "/Game/Blueprints/TestingTimeManagement/BP_CustomTimeManager.BP_CustomTimeManager_C"))
  (bind _output_get (set `self.TimeManager` (`|GetArrayItem` _outactors)))
  (`/Game/Blueprints/TestingTimeManagement/BP_CustomTimeManager.RegisterTimeActor` _output_get self))

(event `/Game/Blueprints/TestingTimeManagement/I_TimeManipulationObject.UpdateTime`
  (params (CurrentTime :type "Float (double-precision)"))
  (`self.ApplySnapshot` CurrentTime))

(fn `ApplySnapshot`
  (params (CurrentTime :type "Float (double-precision)"))
  (`KismetArrayLibrary.Array_Add` (`self.TimeSnapshots`) (make `/Game/Blueprints/TestingTimeManagement/F_TimeSnapshot` (`self.RoundFloat` CurrentTime) (`self.K2_GetActorLocation`) (`self.K2_GetActorRotation`) (`self.IsVisible?`) (`self.HasCollision?`) (`self.GetVelocity`))))

(fn `RoundFloat`
  (params (UnroundedFloat :type "Float (double-precision)"))
  (returns (RoundedFloat :type "Float (double-precision)"))
  (return (/ (`KismetMathLibrary.Conv_IntToDouble` (`KismetMathLibrary.Round` (* UnroundedFloat 10.0))) 10.0)))

(fn `UserConstructionScript`)