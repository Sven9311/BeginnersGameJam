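; BP_CustomTimeManager is a time manager that tracks a shared CurrentTime for registered time actors, with play and rewind states.
; Tick moves CurrentTime forward or backward by delta seconds within zero to MaxTime; forwarding and freezing are unimplemented stubs.
; A looping timer set on BeginPlay sends CurrentTime to every registered actor through UpdateTimeMessage.
; Other code registers actors and switches the state through RegisterTimeActor and UpdateTimeState.
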(event `self.ReceiveBeginPlay`
  (`KismetSystemLibrary.K2_SetTimer` null "ApplySnapshots" 0.1 true))

(event `self.ReceiveTick`
  (params (DeltaSeconds :type "Float (single-precision)"))
  (switch `/Game/Blueprints/TestingTimeManagement/E_TimeState` (`self.ETimeState`)
    (:`NewEnumerator0`
      (set `self.CurrentTime` (`KismetMathLibrary.FClamp` (+ (`GameplayStatics.GetWorldDeltaSeconds`) (`self.CurrentTime`)) 0.0 (`self.MaxTime`))))
    (:`NewEnumerator1`
      (set `self.CurrentTime` (`KismetMathLibrary.FClamp` (- (`self.CurrentTime`) (`GameplayStatics.GetWorldDeltaSeconds`)) 0.0 (`self.MaxTime`))))
    (:`NewEnumerator2`
      (`KismetSystemLibrary.PrintString` "TODO"))
    (:`NewEnumerator3`
      (`KismetSystemLibrary.PrintString` "TODO"))))

(fn `ApplySnapshots`
  (for _array_element (`self.TimeActors`)
    (message `/Game/Blueprints/TestingTimeManagement/I_TimeManipulationObject.UpdateTime` _array_element (`self.CurrentTime`))))

(fn `RegisterTimeActor`
  (params (TimeObject :type "/Game/Blueprints/TestingTimeManagement/BP_TimeObject Object Reference"))
  (`KismetArrayLibrary.Array_AddUnique` (`self.TimeActors`) TimeObject))

(fn `UpdateTimeState`
  (params (NewTimeState :type "/Game/Blueprints/TestingTimeManagement/E_TimeState Enum" :default "NewEnumerator0"))
  (set `self.ETimeState` NewTimeState))

(fn `UserConstructionScript`)