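; BP_Test is a test actor that moves its Cube between two positions when a supplied time reaches EventTime.
; BeginPlay caches the actor location and the TravelPos component's world location as the two endpoints.
; SetTime checks for a narrow window around EventTime, using a DoOnce reset after a delay to avoid repeated triggers.
; ReactToTimer flips the Moved flag and snaps the Cube to the opposite endpoint without sweeping.
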(event `self.ReceiveBeginPlay`
  (set `self.StartPos` (`self.K2_GetActorLocation`))
  (set `self.EndPos` (`SceneComponent.K2_GetComponentLocation` (`self.TravelPos`))))

(event `/Game/Blueprints/I_Test.SetTime`
  (params (Time :type "Float (double-precision)"))
  (if (and (< Time (+ (`self.EventTime`) 0.1)) (> Time (- (`self.EventTime`) 0.1)))
    (`/Engine/EditorBlueprintResources/StandardMacros.DoOnce` false :!label _label
      (:`Completed`
        (`self.ReactToTimer`)
        (`KismetSystemLibrary.Delay` 2.0)
        (goto _label :!via `Reset`)))))

(fn `ReactToTimer`
  (if (`self.Moved?`)
    (`SceneComponent.K2_SetWorldLocation` (`self.Cube`) (`self.StartPos`) false false)
    (set `self.Moved?` false)
    (else
      (`SceneComponent.K2_SetWorldLocation` (`self.Cube`) (`self.EndPos`) false false)
      (set `self.Moved?` true))))

(fn `UserConstructionScript`)