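; Base enemy Blueprint that hands the player to its AI and attacks by spawning a time bubble.
; BeginPlay stores the player character in the AI controller's Blackboard.
; Attack spawns BP_TimeBubble slightly below the enemy and grows it from zero scale with a timeline.
; When the growth finishes, a timer calls DestroySelf, which removes the bubble rather than the enemy.
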(event `self.ReceiveBeginPlay`
  (bind _output_get (set `self.Blackboard` (`AIBlueprintHelperLibrary.GetBlackboard` (`AIBlueprintHelperLibrary.GetAIController` self))))
  (`BlackboardComponent.SetValueAsObject` _output_get (`self.BBKey_PlayerRef`) (`GameplayStatics.GetPlayerCharacter` 0)))

(event `/Game/Blueprints/Interfaces/I_Enemy.Attack`
  (bind (_returnvalue_x _returnvalue_y _returnvalue_z) (`KismetMathLibrary.BreakVector` (`self.K2_GetActorLocation`)))
  (bind _returnvalue (`|SpawnActorFromClass` "/Game/Blueprints/Enemies/BP_TimeBubble.BP_TimeBubble_C" (`KismetMathLibrary.MakeTransform` (`KismetMathLibrary.MakeVector` _returnvalue_x _returnvalue_y (- _returnvalue_z 50.0))) "Undefined" "MultiplyWithRoot" null null))
  (bind _output_get (set `self.TimeBubble` _returnvalue))
  (`self.SetActorScale3D` _output_get (0.0 0.0 0.0))
  (`KismetSystemLibrary.PrintString` "Hello")
  (bind (_direction _bubblealpha) (`Timeline|ScaleUpBubble`)
    (:`Update`
      (`self.SetActorScale3D` (`self.TimeBubble`) (`KismetMathLibrary.VLerp` (0.0 0.0 0.0) (3.0 2.5 3.0) _bubblealpha)))
    (:`Finished`
      (`KismetSystemLibrary.K2_SetTimer` null "DestroySelf" 5.0))))

(fn `DestroySelf`
  (bind _timebubble (`self.TimeBubble`)
    (:`then`
      (`self.K2_DestroyActor` _timebubble))
    (:`else`)))

(fn `UserConstructionScript`)