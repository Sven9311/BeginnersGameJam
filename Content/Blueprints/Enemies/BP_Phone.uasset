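; BP_Phone is an enemy-folder actor that casts a time bubble when the player enters its box trigger.
; The overlap spawns BP_TimeBubble slightly above the phone, and a timeline scales it up from zero to a non-uniform size.
; The Castbubbble flag blocks recasting until a timer after the growth calls DestroySelf, which removes only the bubble and re-arms the phone.
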(event `self.Box.OnComponentBeginOverlap`
  (params (OverlappedComponent :type "PrimitiveComponent Object Reference") (OtherActor :type "Actor Object Reference") (OtherComp :type "PrimitiveComponent Object Reference") (OtherBodyIndex :type Integer) (bFromSweep :type Boolean) (SweepResult :type "HitResult Structure (by ref)"))
  (cast `/Game/Blueprints/Player/BP_Player` OtherActor)
  (if (`self.Castbubbble?`)
    (bind _returnvalue (`|SpawnActorFromClass` "/Game/Blueprints/Enemies/BP_TimeBubble.BP_TimeBubble_C" (`KismetMathLibrary.MakeTransform` (+ (`self.K2_GetActorLocation`) (0.0 0.0 50.0))) "Undefined" "MultiplyWithRoot" null null))
    (bind _output_get (set `self.TimeBubble` _returnvalue))
    (`self.SetActorScale3D` _output_get (0.0 0.0 0.0))
    (bind (_direction _bubblealpha) (`Timeline|Timeline`)
      (:`Update`
        (`self.SetActorScale3D` (`self.TimeBubble`) (`KismetMathLibrary.VLerp` (0.0 0.0 0.0) (4.0 2.5 4.0) _bubblealpha))
        (set `self.Castbubbble?` false))
      (:`Finished`
        (`KismetSystemLibrary.K2_SetTimer` null "DestroySelf" 5.0)))))

(fn `DestroySelf`
  (bind _timebubble (`self.TimeBubble`)
    (:`then`
      (set `self.Castbubbble?` true)
      (`self.K2_DestroyActor` _timebubble))
    (:`else`)))

(fn `UserConstructionScript`)