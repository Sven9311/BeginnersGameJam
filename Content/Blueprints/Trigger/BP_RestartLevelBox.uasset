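; BP_RestartLevelBox is a trigger that shows the death screen when the player overlaps it.
; On overlap with a BP_Player, it creates WB_DeathScreen with the player reference, adds it to the viewport, pauses the game and switches to UI-only input with a visible cursor.
; An unconnected chain that calls Die on the player and sends OnRespawnMessage to all I_PickUp actors never runs.
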(event `self.ReceiveActorBeginOverlap`
  (params (OtherActor :type "Actor Object Reference"))
  (bind _returnvalue (`GameplayStatics.GetPlayerController` 0))
  (bind _asbp_player (cast `/Game/Blueprints/Player/BP_Player` OtherActor))
  (bind _output_get (set `self.PlayerRef` _asbp_player))
  (bind _returnvalue_2 (`|CreateWidget` "/Game/Blueprints/Widgets/WB_DeathScreen.WB_DeathScreen_C" null _output_get))
  (bind _output_get_2 (set `self.DeathScreen` _returnvalue_2))
  (`UserWidget.AddToViewport` _output_get_2 0)
  (`GameplayStatics.SetGamePaused` true)
  (set `PlayerController.bShowMouseCursor` true _returnvalue)
  (`WidgetBlueprintLibrary.SetInputMode_UIOnlyEx` _returnvalue (`self.DeathScreen`)))

(fn `UserConstructionScript`)