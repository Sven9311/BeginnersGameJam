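; BP_SpinningGear is an environment actor that spins continuously, such as a decorative or moving gear.
; Each tick it adds world-space pitch rotation scaled by RotationSpeed and delta seconds, so the spin rate is frame-rate independent.
; A RotationDirection enum switch picks Left or Right, with Left negating the speed.
; The construction script is empty.
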(event `self.ReceiveTick`
  (params (DeltaSeconds :type "Float (single-precision)"))
  (switch `/Game/Blueprints/Environment/E_RotationDirection` (`self.RotationDirection`)
    (:`NewEnumerator0`
      (`self.K2_AddActorWorldRotation` (`KismetMathLibrary.MakeRotator` 0.0 (* (`GameplayStatics.GetWorldDeltaSeconds`) (* -1.0 (`self.RotationSpeed`))))))
    (:`NewEnumerator1`
      (`self.K2_AddActorWorldRotation` (`KismetMathLibrary.MakeRotator` 0.0 (* (`GameplayStatics.GetWorldDeltaSeconds`) (`self.RotationSpeed`)))))))

(fn `UserConstructionScript`)