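; BP_Conveyer is a time-object conveyor belt that pushes the player along world X, with its direction optionally flipped at BeginPlay.
; Box overlap events track whether BP_Player is on the belt.
; While the player is on it, Tick adds LaunchForce to their movement velocity according to the TimeManager state: normal when playing, reversed when rewinding, doubled when forwarding.
; The push is applied every frame without delta-time scaling.
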(event `self.ReceiveBeginPlay`
  (`parent.ReceiveBeginPlay`)
  (if (`self.OppositeDirection?`)
    (set `self.LaunchForce` (* (`self.LaunchForce`) -1.0))))

(event `self.Box.OnComponentBeginOverlap`
  (params (OverlappedComponent :type "PrimitiveComponent Object Reference") (OtherActor :type "Actor Object Reference") (OtherComp :type "PrimitiveComponent Object Reference") (OtherBodyIndex :type Integer) (bFromSweep :type Boolean) (SweepResult :type "HitResult Structure (by ref)"))
  (cast `/Game/Blueprints/Player/BP_Player` OtherActor)
  (set `self.PlayerOnConveyer?` true))

(event `self.Box.OnComponentEndOverlap`
  (params (OverlappedComponent :type "PrimitiveComponent Object Reference") (OtherActor :type "Actor Object Reference") (OtherComp :type "PrimitiveComponent Object Reference") (OtherBodyIndex :type Integer))
  (cast `/Game/Blueprints/Player/BP_Player` OtherActor)
  (set `self.PlayerOnConveyer?` false))

(event `self.ReceiveTick`
  (params (DeltaSeconds :type "Float (single-precision)"))
  (bind _playerref (`self.PlayerRef`))
  (bind _playerref_2 (`self.PlayerRef`))
  (bind _playerref_3 (`self.PlayerRef`))
  (bind (_returnvalue_x _returnvalue_y _returnvalue_z) (`KismetMathLibrary.BreakVector` (`self.GetVelocity` _playerref)))
  (bind (_returnvalue_x_2 _returnvalue_y_2 _returnvalue_z_2) (`KismetMathLibrary.BreakVector` (`self.GetVelocity` _playerref_2)))
  (bind (_returnvalue_x_3 _returnvalue_y_3 _returnvalue_z_3) (`KismetMathLibrary.BreakVector` (`self.GetVelocity` _playerref_3)))
  (if (`self.PlayerOnConveyer?`)
    (switch `/Game/Blueprints/TimeManagement/CustomTypes/E_TimeState` (`/Game/Blueprints/TimeManagement/BP_CustomTimeManager.ETimeState` (`self.TimeManager`))
      (:`NewEnumerator0`
        (set `MovementComponent.Velocity` (`KismetMathLibrary.MakeVector` (+ (`self.LaunchForce`) _returnvalue_x) _returnvalue_y _returnvalue_z) (`Character.CharacterMovement` _playerref)))
      (:`NewEnumerator1`
        (set `MovementComponent.Velocity` (`KismetMathLibrary.MakeVector` (+ (* (`self.LaunchForce`) -1.0) _returnvalue_x_3) _returnvalue_y_3 _returnvalue_z_3) (`Character.CharacterMovement` _playerref_3)))
      (:`NewEnumerator2`
        (set `MovementComponent.Velocity` (`KismetMathLibrary.MakeVector` (+ (* (`self.LaunchForce`) 2.0) _returnvalue_x_2) _returnvalue_y_2 _returnvalue_z_2) (`Character.CharacterMovement` _playerref_2))))))

(fn `UserConstructionScript`
  (`parent.UserConstructionScript`))