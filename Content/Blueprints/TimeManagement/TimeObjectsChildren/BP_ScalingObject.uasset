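; BP_ScalingObject is a time-managed object that shrinks away to nothing from a set event time over a scale duration.
; Each Tick compares TimeManager.CurrentTime with that window and lerps actor scale from full to zero.
; Cylinder collision stays on until the window ends, then switches off.
; Scale and collision derive only from current time, so the object reappears if time moves back.
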(event `self.ReceiveTick`
  (params (DeltaSeconds :type "Float (single-precision)"))
  (if (< (`/Game/Blueprints/TimeManagement/BP_CustomTimeManager.CurrentTime` (`self.TimeManager`)) (`self.EventTime`))
    (`PrimitiveComponent.SetCollisionEnabled` (`self.Cylinder`) "QueryAndPhysics")
    (`self.SetActorScale3D` (1.0 1.0 1.0))
    (elif (> (`/Game/Blueprints/TimeManagement/BP_CustomTimeManager.CurrentTime` (`self.TimeManager`)) (+ (`self.EventTime`) (`self.ScaleDuration`)))
      (`PrimitiveComponent.SetCollisionEnabled` (`self.Cylinder`) "NoCollision")
      (`self.SetActorScale3D` (0.0 0.0 0.0))
      (else
        (`PrimitiveComponent.SetCollisionEnabled` (`self.Cylinder`) "QueryAndPhysics")
        (`self.SetActorScale3D` (`KismetMathLibrary.VLerp` (1.0 1.0 1.0) (0.0 0.0 0.0) (/ (- (`/Game/Blueprints/TimeManagement/BP_CustomTimeManager.CurrentTime` (`self.TimeManager`)) (`self.EventTime`)) (`self.ScaleDuration`))))))))

(fn `UserConstructionScript`
  (`parent.UserConstructionScript`))