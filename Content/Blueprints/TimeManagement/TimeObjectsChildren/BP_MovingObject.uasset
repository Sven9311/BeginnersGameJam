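; BP_MovingObject is a time-managed child actor that moves between two points over a timed window.
; On BeginPlay it records its own location as the start and its Scene component's world location as the end.
; Each tick it derives position directly from the TimeManager's current time, clamping outside the EventTime to EventTime plus MoveDuration window and linearly interpolating inside it.
; It also updates an IsMoving flag.
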(event `self.ReceiveBeginPlay`
  (`parent.ReceiveBeginPlay`)
  (set `self.StartPos` (`self.K2_GetActorLocation`))
  (set `self.EndPos` (`SceneComponent.K2_GetComponentLocation` (`self.Scene`))))

(event `self.ReceiveTick`
  (params (DeltaSeconds :type "Float (single-precision)"))
  (`parent.ReceiveTick` DeltaSeconds)
  (if (< (`/Game/Blueprints/TimeManagement/BP_CustomTimeManager.CurrentTime` (`self.TimeManager`)) (`self.EventTime`))
    (set `self.isMoving?` false)
    (`self.K2_SetActorLocation` (`self.StartPos`))
    (elif (> (`/Game/Blueprints/TimeManagement/BP_CustomTimeManager.CurrentTime` (`self.TimeManager`)) (+ (`self.EventTime`) (`self.MoveDuration`)))
      (set `self.isMoving?` false)
      (`self.K2_SetActorLocation` (`self.EndPos`))
      (else
        (set `self.isMoving?` true)
        (`self.K2_SetActorLocation` (`KismetMathLibrary.VLerp` (`self.StartPos`) (`self.EndPos`) (/ (- (`/Game/Blueprints/TimeManagement/BP_CustomTimeManager.CurrentTime` (`self.TimeManager`)) (`self.EventTime`)) (`self.MoveDuration`))))))))

(fn `ApplySnapshot`
  (params (CurrentTime :type "Float (double-precision)"))
  (`parent.ApplySnapshot` CurrentTime))

(fn `UserConstructionScript`
  (`parent.UserConstructionScript`))