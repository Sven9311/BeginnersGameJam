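; BP_RotatingWall is a time-affected wall that spins continuously around its local pitch axis.
; BeginPlay calls the parent and flips RotationSpeed when InverseRotation is set.
; Each Tick reads the TimeManager's time state to run the spin normally, reversed, at double speed or stopped, scaled by world delta seconds.
; Rewind simply negates the speed instead of replaying recorded transforms.
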(event `self.ReceiveBeginPlay`
  (`parent.ReceiveBeginPlay`)
  (if (`self.InverseRotation?`)
    (set `self.RotationSpeed` (* (`self.RotationSpeed`) -1.0))))

(event `self.ReceiveTick`
  (params (DeltaSeconds :type "Float (single-precision)"))
  (switch `/Game/Blueprints/TimeManagement/CustomTypes/E_TimeState` (`/Game/Blueprints/TimeManagement/BP_CustomTimeManager.ETimeState` (`self.TimeManager`))
    (:`NewEnumerator0`
      (set `self.ManipulatedRotationSpeed` (`self.RotationSpeed`)))
    (:`NewEnumerator1`
      (set `self.ManipulatedRotationSpeed` (* (`self.RotationSpeed`) -1.0)))
    (:`NewEnumerator2`
      (set `self.ManipulatedRotationSpeed` (* (`self.RotationSpeed`) 2.0)))
    (:`NewEnumerator3`
      (set `self.ManipulatedRotationSpeed` 0.0)))
  (`SceneComponent.K2_AddLocalRotation` (`self.Scene`) (`KismetMathLibrary.MakeRotator` 0.0 (* (`GameplayStatics.GetWorldDeltaSeconds`) (`self.ManipulatedRotationSpeed`))) false false))

(fn `UserConstructionScript`
  (`parent.UserConstructionScript`))