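; Player controller for a side-view platformer, turning Enhanced Input into BP_Player movement, pause menu and time powers.
; Handles multi-jumps, slide gravity and double-tap dashes with limited air uses and speed-based strength.
; Tick raises max walk speed to preserve momentum, flags input changes for friction checks, and line-traces walls for slowing and wall jumps.
; Freeze, rewind and forward inputs toggle BP_CustomTimeManager states, gated by the player's time fuel.
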(event `self.ReceiveBeginPlay`
  ;[0 0 0 0.5] SettingUp Variables
  (bind _asbp_player (cast `/Game/Blueprints/Player/BP_Player` (`self.K2_GetPawn`)))
  (set `self.PlayerRef` _asbp_player)
  (`EnhancedInputSubsystemInterface.AddMappingContext` (subsystem `EnhancedInputLocalPlayerSubsystem`) "/Game/Input/IMC_Default.IMC_Default" 0 (struct))
  (bind _outactors (`GameplayStatics.GetAllActorsOfClass` "/Game/Blueprints/TimeManagement/BP_CustomTimeManager.BP_CustomTimeManager_C"))
  (set `self.CustomTimeManager` (`|GetArrayItem` _outactors))
  (set `self.InitialDashSpeed` (`/Game/Blueprints/Player/BP_Player.DashSpeed` (`self.PlayerRef`))))

(event `EnhancedInput|/Game/Input/Inputs/IA_Move`
  (params (ActionValue :type "Vector2D Structure") (ElapsedSeconds :type "Float (double-precision)") (TriggeredSeconds :type "Float (double-precision)") (InputAction :type "InputAction Object Reference" :default "/Game/Input/Inputs/IA_Move.IA_Move"))
  ;[0 0 0 0.5] MoveInput
  (:`Triggered`
    (set `self.CurrentInputValue` ActionValue_X)
    (`Pawn.AddMovementInput` (`self.PlayerRef`) (`KismetMathLibrary.MakeVector` ActionValue_X) 1.0 false))
  (:`Started`
    (set `self.isRunning?` true)
    (`/Game/Blueprints/Player/BP_Player.CheckGroundFriction` (`self.PlayerRef`)))
  (:`Completed`
    (set `self.isRunning?` false)
    (`/Game/Blueprints/Player/BP_Player.CheckGroundFriction` (`self.PlayerRef`))))

(event `EnhancedInput|/Game/Input/Inputs/IA_Jump`
  (params (ActionValue :type Boolean) (ElapsedSeconds :type "Float (double-precision)") (TriggeredSeconds :type "Float (double-precision)") (InputAction :type "InputAction Object Reference" :default "/Game/Input/Inputs/IA_Jump.IA_Jump"))
  (bind _playerref (`self.PlayerRef`))
  (bind _playerref_2 (`self.PlayerRef`))
  (bind _jumpcount (`self.JumpCount`))
  ;[0 0 0 0.5] JumpInput
  (:`Started`
    (if (not (`/Game/Blueprints/Player/BP_Player.IsOnJumpPad?` _playerref))
      (if (`self.WallJump?`)
        (`self.HandleWallJump`)
        (else
          (`/Engine/EditorBlueprintResources/StandardMacros.IncrementInt` _jumpcount
            (:`  `
              (if (> _jumpcount 1)
                (set `CharacterMovementComponent.JumpZVelocity` (`self.decreasedJumpVelocity`) (`Character.CharacterMovement` (`self.PlayerRef`)))
                (else
                  (set `CharacterMovementComponent.JumpZVelocity` (`/Game/Blueprints/Player/BP_Player.JumpVelocity` _playerref_2) (`Character.CharacterMovement` _playerref_2))))
              (`Character.Jump` (`self.PlayerRef`))))))
      (else
        (`/Game/Blueprints/Player/BP_Player.UseJumpPad` _playerref)))))

(event `EnhancedInput|/Game/Input/Inputs/IA_TapLeft`
  (params (ActionValue :type Boolean) (ElapsedSeconds :type "Float (double-precision)") (TriggeredSeconds :type "Float (double-precision)") (InputAction :type "InputAction Object Reference" :default "/Game/Input/Inputs/IA_TapLeft.IA_TapLeft"))
  ;[0 0 0 0.5] MoveInput
  (:`Started`
    (if (`self.CanDash?`)
      (set `self.DashDirection` -1.0)
      (`self.HandleDash` (`self.CheckDashWindow` (`self.LastLeftPressTime`)))
      (set `self.LastLeftPressTime` (`GameplayStatics.GetTimeSeconds`)))))

(event `EnhancedInput|/Game/Input/Inputs/IA_Pause`
  (params (ActionValue :type Boolean) (ElapsedSeconds :type "Float (double-precision)") (TriggeredSeconds :type "Float (double-precision)") (InputAction :type "InputAction Object Reference" :default "/Game/Input/Inputs/IA_Pause.IA_Pause"))
  ;[0 0 0 0.5] PauseMenu
  (:`Started`
    (`/Engine/EditorBlueprintResources/StandardMacros.IsValid` (`self.PauseMenuRef`)
      (:`Is Valid`
        _)
      (:`Is Not Valid`
        (bind _returnvalue (`|CreateWidget` "/Game/Blueprints/Widgets/WB_PauseMenu.WB_PauseMenu_C"))
        (set `self.PauseMenuRef` _returnvalue)))
    (if (`GameplayStatics.IsGamePaused`)
      (`self.HidePauseWindow`)
      (else
        (`self.ShowPauseWindow`)))))

(event `EnhancedInput|/Game/Input/Inputs/IA_TapRight`
  (params (ActionValue :type Boolean) (ElapsedSeconds :type "Float (double-precision)") (TriggeredSeconds :type "Float (double-precision)") (InputAction :type "InputAction Object Reference" :default "/Game/Input/Inputs/IA_TapRight.IA_TapRight"))
  ;[0 0 0 0.5] MoveInput
  (:`Started`
    (if (`self.CanDash?`)
      (set `self.DashDirection` 1.0)
      (`self.HandleDash` (`self.CheckDashWindow` (`self.LastRightPressTime`)))
      (set `self.LastRightPressTime` (`GameplayStatics.GetTimeSeconds`)))))

(event `self.ReceiveTick`
  (params (DeltaSeconds :type "Float (single-precision)"))
  (`self.AdjustMovementSpeed`)
  (`self.CheckForInputChange`)
  (`self.CanWallJump?`))

(event `EnhancedInput|/Game/Input/Inputs/IA_FreezeTime`
  (params (ActionValue :type Boolean) (ElapsedSeconds :type "Float (double-precision)") (TriggeredSeconds :type "Float (double-precision)") (InputAction :type "InputAction Object Reference" :default "/Game/Input/Inputs/IA_FreezeTime.IA_FreezeTime"))
  ;[0 0 0 0.5] FreezeTime
  (:`Started`
    (switch `/Game/Blueprints/TimeManagement/CustomTypes/E_TimeState` (`/Game/Blueprints/TimeManagement/BP_CustomTimeManager.ETimeState` (`self.CustomTimeManager`))
      (:`NewEnumerator0`
        (if (`self.HasEnoughFuel?`) :!label _label
          (`/Game/Blueprints/TimeManagement/BP_CustomTimeManager.UpdateTimeState` (`self.CustomTimeManager`) "NewEnumerator3")
          (else
            (`/Game/Blueprints/TimeManagement/BP_CustomTimeManager.UpdateTimeState` (`self.CustomTimeManager`) "NewEnumerator0" :!label _label_2))))
      (:`NewEnumerator1`
        (goto _label))
      (:`NewEnumerator2`
        (goto _label))
      (:`NewEnumerator3`
        (goto _label_2)))))

(event `EnhancedInput|/Game/Input/Inputs/IA_Slide`
  (params (ActionValue :type Boolean) (ElapsedSeconds :type "Float (double-precision)") (TriggeredSeconds :type "Float (double-precision)") (InputAction :type "InputAction Object Reference" :default "/Game/Input/Inputs/IA_Slide.IA_Slide"))
  (bind _playerref (`self.PlayerRef`))
  (:`Started`
    (set `self.SlidePressed?` true)
    (set `CharacterMovementComponent.GravityScale` (`self.GravityScaleWhileS`) (`Character.CharacterMovement` (`self.PlayerRef`))))
  (:`Completed`
    (set `self.SlidePressed?` false)
    (set `CharacterMovementComponent.GravityScale` (`/Game/Blueprints/Player/BP_Player.GravityScale` _playerref) (`Character.CharacterMovement` _playerref))))

(event `EnhancedInput|/Game/Input/Inputs/IA_ReverseTime`
  (params (ActionValue :type Boolean) (ElapsedSeconds :type "Float (double-precision)") (TriggeredSeconds :type "Float (double-precision)") (InputAction :type "InputAction Object Reference" :default "/Game/Input/Inputs/IA_ReverseTime.IA_ReverseTime"))
  ;[0 0 0 0.5] RewindInput
  (:`Started`
    (switch `/Game/Blueprints/TimeManagement/CustomTypes/E_TimeState` (`/Game/Blueprints/TimeManagement/BP_CustomTimeManager.ETimeState` (`self.CustomTimeManager`))
      (:`NewEnumerator0`
        (if (`self.HasEnoughFuel?`) :!label _label_3
          (`/Game/Blueprints/TimeManagement/BP_CustomTimeManager.UpdateTimeState` (`self.CustomTimeManager`) "NewEnumerator1")
          (else
            (`/Game/Blueprints/TimeManagement/BP_CustomTimeManager.UpdateTimeState` (`self.CustomTimeManager`) "NewEnumerator0" :!label _label_4))))
      (:`NewEnumerator1`
        (goto _label_4))
      (:`NewEnumerator2`
        (goto _label_3))
      (:`NewEnumerator3`
        (goto _label_3)))))

(event `EnhancedInput|/Game/Input/Inputs/IA_ForwardTime`
  (params (ActionValue :type Boolean) (ElapsedSeconds :type "Float (double-precision)") (TriggeredSeconds :type "Float (double-precision)") (InputAction :type "InputAction Object Reference" :default "/Game/Input/Inputs/IA_ForwardTime.IA_ForwardTime"))
  ;[0 0 0 0.5] ForwardTime
  (:`Started`
    (switch `/Game/Blueprints/TimeManagement/CustomTypes/E_TimeState` (`/Game/Blueprints/TimeManagement/BP_CustomTimeManager.ETimeState` (`self.CustomTimeManager`))
      (:`NewEnumerator0`
        (if (`self.HasEnoughFuel?`) :!label _label_5
          (`/Game/Blueprints/TimeManagement/BP_CustomTimeManager.UpdateTimeState` (`self.CustomTimeManager`) "NewEnumerator2")
          (else
            (`/Game/Blueprints/TimeManagement/BP_CustomTimeManager.UpdateTimeState` (`self.CustomTimeManager`) "NewEnumerator0" :!label _label_6))))
      (:`NewEnumerator1`
        (goto _label_5))
      (:`NewEnumerator2`
        (goto _label_6))
      (:`NewEnumerator3`
        (goto _label_5)))))

(fn `AdjustMovementSpeed`
  (bind _movementspeed (`/Game/Blueprints/Player/BP_Player.MovementSpeed` (`self.PlayerRef`)))
  (bind _velocity_x (`KismetMathLibrary.BreakVector` (`MovementComponent.Velocity` (`Character.CharacterMovement` (`self.PlayerRef`)))))
  (bind _returnvalue (`KismetMathLibrary.Abs` _velocity_x))
  (if (> _returnvalue _movementspeed)
    (set `CharacterMovementComponent.MaxWalkSpeed` _returnvalue (`Character.CharacterMovement` (`self.PlayerRef`)))
    (else
      (set `CharacterMovementComponent.MaxWalkSpeed` _movementspeed (`Character.CharacterMovement` (`self.PlayerRef`))))))

(fn `CanDash?`
  (returns (ReturnValue :type Boolean))
  (return (or (and (and (`NavMovementComponent.IsFalling` (`Character.CharacterMovement` (`self.PlayerRef`))) (< (`self.CurrentDashesAir`) (`self.MaxDashesAir`))) (`self.DashAvailable?`)) (and (`CharacterMovementComponent.IsWalking` (`Character.CharacterMovement` (`self.PlayerRef`))) (`self.DashAvailable?`)))))

(fn `CanWallJump?`
  (if (`self.isPlayerFalling?`)
    (if (`self.CheckForWallJump`)
      (bind _output_get (set `self.WallJump?` true))
      (`self.InitialWallVelocity` (!= _output_get (`self.PreviousWallJumpState`)))
      (`self.HandleSlowOnWall`)
      (set `self.PreviousWallJumpState` _output_get)
      (else
        (bind _output_get_2 (set `self.WallJump?` false))
        (set `self.PreviousWallJumpState` _output_get_2)))
    (else
      (set `self.WallJump?` false))))

(fn `CheckDashWindow`
  (params (LastTimeKeyPressed :type "Float (double-precision)"))
  (returns (ReturnValue :type Boolean))
  (return (<= (- (`GameplayStatics.GetTimeSeconds`) LastTimeKeyPressed) (`self.DoubleTapThreshhold`))))

(fn `CheckForInputChange`
  (if (not (== (`self.CurrentInputValue`) (`self.LastInputValue`)))
    (`self.OnInputChange`))
  (set `self.LastInputValue` (`self.CurrentInputValue`)))

(fn `CheckForWallJump`
  (returns (`NextToWall?` :type Boolean))
  (locals (Hit1 :type Boolean :default false) (Hit2 :type Boolean :default false))
  (bind _playerref (`self.PlayerRef`))
  (bind _playerref_2 (`self.PlayerRef`))
  (bind _returnvalue_x (`KismetMathLibrary.BreakVector` (`self.K2_GetActorLocation` (`self.PlayerRef`))))
  (bind _returnvalue_x_2 (`KismetMathLibrary.BreakVector` (`self.K2_GetActorLocation` (`self.PlayerRef`))))
  (bind _returnvalue (or (`local.Hit1`) (`local.Hit2`)))
  (bind _returnvalue_2 (+ (`self.K2_GetActorLocation` _playerref_2) (0.0 0.0 -30.0)))
  (bind _returnvalue_3 (+ (`self.K2_GetActorLocation` _playerref) (0.0 0.0 -50.0)))
  (bind (_outhit _returnvalue_4) (`KismetSystemLibrary.LineTraceSingle` _returnvalue_3 (+ _returnvalue_3 (* (`self.GetActorForwardVector` _playerref) (`self.WallCheckDistance`))) "TraceTypeQuery3"))
  (bind _output_get (set `local.Hit1` _returnvalue_4))
  (if _output_get
    (if (> (.x (`.Location` (`GameplayStatics.BreakHitResult` _outhit))) _returnvalue_x_2)
      (set `self.CurrentWallPosition` "NewEnumerator1")
      (else
        (set `self.CurrentWallPosition` "NewEnumerator0"))))
  (bind (_outhit_2 _returnvalue_5) (`KismetSystemLibrary.LineTraceSingle` _returnvalue_2 (+ _returnvalue_2 (* (* (`self.GetActorForwardVector` _playerref_2) -1.0) (`self.WallCheckDistance`))) "TraceTypeQuery3"))
  (bind _output_get_2 (set `local.Hit2` _returnvalue_5))
  (if _output_get_2
    (if (> (.x (`.Location` (`GameplayStatics.BreakHitResult` _outhit_2))) _returnvalue_x)
      (set `self.CurrentWallPosition` "NewEnumerator1")
      (else
        (set `self.CurrentWallPosition` "NewEnumerator0"))))
  (if (not _returnvalue)
    (set `self.CurrentWallPosition` "NewEnumerator2"))
  (return _returnvalue))

(fn `HandleDash`
  (params (Condition :type Boolean))
  (bind _playerref (`self.PlayerRef`))
  (bind _playerref_2 (`self.PlayerRef`))
  (bind (_returnvalue_x _returnvalue_y _returnvalue_z) (`KismetMathLibrary.BreakVector` (`self.GetActorForwardVector` _playerref)))
  (bind _returnvalue_x_2 (`KismetMathLibrary.BreakVector` (`self.GetVelocity` (`self.PlayerRef`))))
  (bind _returnvalue_x_3 (`KismetMathLibrary.BreakVector` (`self.GetVelocity` _playerref_2)))
  (bind _dashspeed (`/Game/Blueprints/Player/BP_Player.DashSpeed` _playerref))
  (bind _returnvalue (`KismetMathLibrary.Abs` _returnvalue_x_3))
  (bind _returnvalue_2 (`KismetMathLibrary.Abs` _returnvalue_x_2))
  (if Condition
    (if (< (`/Game/Blueprints/Player/BP_Player.DashSpeed` _playerref_2) _returnvalue)
      (if (> _returnvalue_2 (`/Game/Blueprints/Player/BP_Player.MaxMovementSpeed` (`self.PlayerRef`)))
        (set `/Game/Blueprints/Player/BP_Player.DashSpeed` (* _returnvalue_2 (`self.DashChangeValue`)) (`self.PlayerRef`))
        (else
          (set `/Game/Blueprints/Player/BP_Player.DashSpeed` _returnvalue (`self.PlayerRef`))))
      (else
        (set `/Game/Blueprints/Player/BP_Player.DashSpeed` (`self.InitialDashSpeed`) (`self.PlayerRef`))))
    (if (< (`self.DashDirection`) 0.0)
      (`Character.LaunchCharacter` _playerref (`KismetMathLibrary.MakeVector` (* -1.0 _dashspeed) _returnvalue_y _returnvalue_z) true false)
      (else
        (`Character.LaunchCharacter` _playerref (`KismetMathLibrary.MakeVector` (* 1.0 _dashspeed) _returnvalue_y _returnvalue_z) true false)))
    (if (`NavMovementComponent.IsFalling` (`Character.CharacterMovement` (`self.PlayerRef`)))
      (`/Engine/EditorBlueprintResources/StandardMacros.IncrementInt` (`self.CurrentDashesAir`)
        (:`  `
          _)))
    (set `self.DashAvailable?` true))
  (return))

(fn `HandleSlowOnWall`
  (bind _charactermovement (`Character.CharacterMovement` (`self.PlayerRef`)))
  (set `MovementComponent.Velocity` (`KismetMathLibrary.VInterpTo_Constant` (`MovementComponent.Velocity` _charactermovement) (0.0 0.0 0.0) (`GameplayStatics.GetWorldDeltaSeconds`) (`self.WallFriction`)) _charactermovement))

(fn `HandleWallJump`
  (switch `/Game/Blueprints/Controller/E_WallPosition` (`self.CurrentWallPosition`)
    (:`NewEnumerator0`
      (`Character.LaunchCharacter` (`self.PlayerRef`) (`KismetMathLibrary.MakeVector` (* (`self.WallJumpForce`) -1.0) 0.0 1000.0) true true)
      (`self.K2_SetActorRotation` (`self.PlayerRef`) (`KismetMathLibrary.MakeRotator` 0.0) false))
    (:`NewEnumerator1`
      (`Character.LaunchCharacter` (`self.PlayerRef`) (`KismetMathLibrary.MakeVector` (`self.WallJumpForce`) 0.0 1000.0) true true)
      (`self.K2_SetActorRotation` (`self.PlayerRef`) (`KismetMathLibrary.MakeRotator` 0.0 180.0) false))))

(fn `HasEnoughFuel?`
  (returns (ReturnValue :type Boolean))
  (return (>= (`/Game/Blueprints/Player/BP_Player.CurrentTimeFuel` (`self.PlayerRef`)) (`self.FuelThreshhold`))))

(fn `HidePauseWindow`
  (bind _returnvalue (`GameplayStatics.GetPlayerController` 0))
  (`Widget.RemoveFromParent` (`self.PauseMenuRef`))
  (`GameplayStatics.SetGamePaused` false)
  (set `PlayerController.bShowMouseCursor` false _returnvalue)
  (`WidgetBlueprintLibrary.SetInputMode_GameOnly` _returnvalue))

(fn `InitialWallVelocity`
  (params (Condition :type Boolean))
  (bind _playerref (`self.PlayerRef`))
  (bind (_returnvalue_x _returnvalue_y _returnvalue_z) (`KismetMathLibrary.BreakVector` (`self.GetVelocity` (`self.PlayerRef`))))
  (if Condition
    (if (< _returnvalue_z 0.0)
      (`Character.LaunchCharacter` _playerref (`self.WallDownwardsVelocity`) false false)
      (else
        (`Character.LaunchCharacter` _playerref (`self.WallUpwardsVelocity`) false false)))))

(fn `isPlayerFalling?`
  (returns (ReturnValue :type Boolean))
  (return (`NavMovementInterface.IsFalling` (`Character.CharacterMovement` (`self.PlayerRef`)))))

(fn `OnInputChange`
  (set `self.inputChanged?` true)
  (`/Game/Blueprints/Player/BP_Player.CheckGroundFriction` (`self.PlayerRef`))
  (`KismetSystemLibrary.K2_SetTimer` null "ResetInputChange" 0.2))

(fn `ResetDashCooldown`
  (set `self.DashAvailable?` true))

(fn `ResetInputChange`
  (set `self.inputChanged?` false)
  (`/Game/Blueprints/Player/BP_Player.CheckGroundFriction` (`self.PlayerRef`)))

(fn `ShowPauseWindow`
  (bind _returnvalue (`GameplayStatics.GetPlayerController` 0))
  (`UserWidget.AddToViewport` (`self.PauseMenuRef`) 0)
  (`GameplayStatics.SetGamePaused` true)
  (set `PlayerController.bShowMouseCursor` true _returnvalue)
  (`WidgetBlueprintLibrary.SetInputMode_GameAndUIEx` _returnvalue (`self.PauseMenuRef`)))

(fn `UserConstructionScript`)